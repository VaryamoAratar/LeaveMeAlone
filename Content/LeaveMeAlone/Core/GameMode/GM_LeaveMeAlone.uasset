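; Game mode for LeaveMeAlone that runs the match countdown and reacts to the player's death.
; A looping one-second timer decrements GameTime and, at zero, stops itself and calls ViewPortMenu if an IsValid check fails.
; The player health component's OnDeath event also stops the timer and calls ViewPortMenu after a short delay.
; ViewPortMenu takes a widget parameter but has an empty body here.
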(event Custom|CustomEvent
  (bind _output_get (Variables|Default|SetGameTime (- (Variables|Default|GetGameTime) 1)))
  (if (== _output_get 0)
    (Utilities|IsValid 0
      (:Is%20Not%20Valid
        (Utilities|Time|ClearandInvalidateTimerbyHandle (Variables|Default|GetGame%20Timer%20Handle))
        (CallFunction|ViewPortMenu)))))

(event Custom|CustomEvent_1
  (Utilities|Time|ClearandInvalidateTimerbyHandle (Variables|Default|GetGame%20Timer%20Handle))
  (Utilities|FlowControl|Delay 3.0)
  (CallFunction|ViewPortMenu))

(event EventBeginPlay
  (Utilities|FlowControl|Sequence
    (:then_0
      (bind _returnvalue (Utilities|Time|SetTimerbyEvent (delegate Custom|CustomEvent) 1.0 true))
      (Variables|Default|SetGame%20Timer%20Handle _returnvalue))
    (:then_1
      (EventDispatchers|BindEventtoOnDeath (Actor|GetComponentbyClass (Game|GetPlayerCharacter 0) "/Script/LeaveMeAlone.LMAHealthComponent") (delegate Custom|CustomEvent_1)))))

(event EventTick
  (params (DeltaSeconds :type Float%20%28single-precision%29)))

(fn ConstructionScript)

(fn ViewPortMenu
  (params (WBP :type User%20Widget%20Class%20Reference))
  (return 0))